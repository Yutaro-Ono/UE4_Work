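; BP_Enemy_1 is an enemy that wanders randomly within the bounds of a BoxMoveArea reference.
; On BeginPlay it teleports to a random XY point in that box, keeping its own Z.
; It then loops AI MoveTo to new random points, pausing a random few seconds after each success or failure.
; GetRandomLocation samples the box's collision bounds, returning the world origin if the area is invalid.
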(event `self.ReceiveBeginPlay`
  ;[1 1 1] 初期座標のセット
  ;;[1 1 1] ランダム座標を取得 ※Ｚは無視
  (bind _location (`self.Get Random Location`))
  (`self.K2_SetActorLocation` (`KismetMathLibrary.MakeVector` (.x _location) (.y _location) (.z (`self.K2_GetActorLocation`))))
  ;[1 1 1] ランダム移動ループ（目的地到達後2,3秒待機）
  (bind _location_2 (`self.Get Random Location` :!label _label))
  (`AITask_MoveTo.AIMoveTo` (`AIBlueprintHelperLibrary.GetAIController` self) (`KismetMathLibrary.MakeVector` (.x _location_2) (.y _location_2) (.z (`self.K2_GetActorLocation`))) null -1.0 "Default" "Default" true false
    (:`OnRequestFailed`
      _)
    (:`OnMoveFinished`
      _))
  ;;[1 1 1] 設定秒数の間からランダムに待機時間をセット
  (`KismetSystemLibrary.Delay` (`KismetMathLibrary.RandomFloatInRange` 2.0 5.0))
  (goto _label))

(fn `Get Random Location`
  (returns (Location :type "Vector Structure"))
  (bind _box_movearea (`self.Box_MoveArea`))
  (bind (_origin _boxextent) (`KismetSystemLibrary.GetComponentBounds` (`TriggerBase.CollisionComponent` _box_movearea)))
  ;[1 1 1] ランダムな座標を取得
  (`/Engine/EditorBlueprintResources/StandardMacros.IsValid` _box_movearea
    (:`Is Valid`
      (return (`KismetMathLibrary.RandomPointInBoundingBox` _origin _boxextent)))
    (:`Is Not Valid`
      (return (0.0 0.0 0.0)))))

(fn `UserConstructionScript`)