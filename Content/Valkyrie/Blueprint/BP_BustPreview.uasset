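; BP_BustPreview is a preview actor that shows bust morph targets side by side on skeletal meshes.
; The construction script adds seventeen skeletal mesh components in two staggered rows, each with a text label above it from MorphsTargetList.
; On BeginPlay, each stored mesh gets the morph target at its index in a separate Morphs array set to full weight.
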(event `self.ReceiveBeginPlay`
  (for (_array_element _array_index) (`self.AllMeshes`)
    (`SkeletalMeshComponent.SetMorphTarget` _array_element (`KismetStringLibrary.Conv_StringToName` (`|GetArrayItem` (`self.Morphs`) _array_index)) 1.0 true)))

(fn `UserConstructionScript`
  (locals (SkelMeshComponentLocation :type "Vector Structure" :default (0.0 0.0 0.0)) (MorphsTargetList :type "Array of String") (LoopIndex :type Integer))
  (bind _skelmeshcomponentlocation (`local.SkelMeshComponentLocation`))
  (for _index (range 17)
    (bind _output_get (set `local.LoopIndex` _index))
    (bind _returnvalue (select `bool` (<= _output_get 8) :`false` (+ _skelmeshcomponentlocation (-720.0 100.0 0.0)) :`true` _skelmeshcomponentlocation))
    (bind _returnvalue_2 (`AddComponent|NODE_AddSkeletalMeshComponent-0` :`RelativeTransform` (`KismetMathLibrary.MakeTransform` _returnvalue)))
    (`KismetArrayLibrary.Array_Add` (`self.AllMeshes`) _returnvalue_2)
    (bind _returnvalue_3 (`AddComponent|NODE_AddTextRenderComponent-0` :`RelativeTransform` (`KismetMathLibrary.MakeTransform` (+ _returnvalue (0.0 0.0 100.0)) (struct :`Yaw` 90.0))))
    (`TextRenderComponent.K2_SetText` _returnvalue_3 (`KismetTextLibrary.Conv_StringToText` (`|GetArrayItem` (`local.MorphsTargetList`) (`local.LoopIndex`))))
    (set `local.SkelMeshComponentLocation` (+ _skelmeshcomponentlocation (80.0 0.0 0.0)))))